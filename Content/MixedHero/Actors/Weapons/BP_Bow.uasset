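; VR bow actor that BP_MotionController can pick up and drop, firing arrows drawn with the right hand.
; Right-hand overlap with the Sphere enables firing; Prepare spawns an Arrow_tile on the muzzle and attaches the Sphere to that hand.
; While ready, Tick aligns the bow along the Sphere-to-muzzle line and offsets the arrow.
; Fire derives arrow speed from muzzle and Sphere forward vectors, releases it, and resets the Sphere.
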(event `self.ReceiveTick`
  (params (DeltaSeconds :type "Float (single-precision)"))
  (bind _staticmeshcomponent (`self.StaticMeshComponent`))
  (bind _relativelocation (`SceneComponent.RelativeLocation` (`self.Sphere`)))
  (bind (_returnvalue_roll _returnvalue_pitch _returnvalue_yaw) (`KismetMathLibrary.BreakRotator` (`KismetMathLibrary.FindLookAtRotation` (`SceneComponent.K2_GetComponentLocation` (`self.Sphere`)) (`SceneComponent.K2_GetComponentLocation` (`self.MuzzleScene`)))))
  (if (`self.ready`)
    (`|ExecutionSequence`
      (:`then_0`
        (`SceneComponent.K2_SetRelativeRotation` _staticmeshcomponent (`KismetMathLibrary.MakeRotator` (- _returnvalue_roll 90.0) _returnvalue_pitch _returnvalue_yaw) false false)
        (`SceneComponent.K2_AddRelativeRotation` :`self` _staticmeshcomponent))
      (:`then_1`
        (`SceneComponent.K2_AddRelativeLocation` (`/Game/MixedHero/Actors/Weapons/arrow_tile.DefaultSceneRoot` (`self.Arrow`)) _relativelocation false false)
        (`KismetSystemLibrary.PrintString` (`KismetStringLibrary.Conv_VectorToString` _relativelocation) true true (struct :`R` 1.0 :`G` 0.041667 :`B` 0.181363 :`A` 1.0) 0.01)))))

(event `/Game/VirtualRealityBP/Blueprints/PickupActorInterface.Pickup`
  (params (AttachTo :type "SceneComponent Object Reference"))
  (`PrimitiveComponent.SetSimulatePhysics` (`self.StaticMeshComponent`) false)
  (`SceneComponent.K2_AttachToComponent` (`self.K2_GetRootComponent`) AttachTo "Pickup" "SnapToTarget" "KeepWorld" "KeepWorld" false)
  (`SceneComponent.K2_SetRelativeLocationAndRotation` (`self.StaticMeshComponent`) (-6.0 0.0 6.0) (struct :`Roll` -90.0) false false))

(event `/Game/VirtualRealityBP/Blueprints/PickupActorInterface.Drop`
  (`PrimitiveComponent.SetSimulatePhysics` (`self.StaticMeshComponent`) true)
  (`self.K2_DetachFromActor` "KeepWorld" "KeepWorld" "KeepWorld"))

(event `EventFire`
  (`self.Fire`))

(event `self.Sphere.OnComponentBeginOverlap`
  (params (OverlappedComponent :type "PrimitiveComponent Object Reference") (OtherActor :type "Actor Object Reference") (OtherComp :type "PrimitiveComponent Object Reference") (OtherBodyIndex :type Integer) (bFromSweep :type Boolean) (SweepResult :type "HitResult Structure (by ref)"))
  (bind _asbp_hero_motion_controller (cast `/Game/MixedHero/Controller/BP_HeroMotionController` OtherActor))
  (if (`|EnumEquality` (`/Game/MixedHero/Controller/BP_HeroMotionController.Hand` _asbp_hero_motion_controller) "Right")
    (set `self.hand` _asbp_hero_motion_controller)
    (set `self.canFire` true)
    (`KismetSystemLibrary.PrintString` "Ay Elledi Bu")))

(event `EventPrepare`
  (`self.Prepare`))

(fn `Fire`
  (bind _sphere (`self.Sphere`))
  (bind _arrow (`self.Arrow`))
  (bind _returnvalue_x (`KismetMathLibrary.BreakVector` (- (`SceneComponent.GetForwardVector` (`self.MuzzleScene`)) (`SceneComponent.GetForwardVector` (`self.Sphere`)))))
  (bind _returnvalue (/ (`KismetMathLibrary.FClamp` _returnvalue_x 0.0 100.0) 100.0))
  (if (`self.canFire`)
    (`/Game/MixedHero/Actors/Weapons/arrow_tile.ChangeSpeed` (`self.Arrow`) _returnvalue)
    (`self.K2_DetachFromActor` _arrow "KeepWorld" "KeepWorld" "KeepWorld")
    (`/Game/MixedHero/Actors/Weapons/arrow_tile.Activate` _arrow)
    (set `self.Arrow` null)
    (set `self.canFire` false)
    (set `self.ready` false)
    (`KismetSystemLibrary.PrintString` (`KismetStringLibrary.Conv_DoubleToString` _returnvalue) true true (struct :`R` 1.0 :`B` 0.102586 :`A` 1.0))
    (`SceneComponent.K2_AttachToComponent` _sphere (`self.StaticMeshComponent`) "None" "SnapToTarget" "SnapToTarget" "KeepWorld" true)
    (`SceneComponent.K2_SetRelativeLocation` _sphere (-30.0 0.0 0.0) false false)))

(fn `Prepare`
  (bind (_returnvalue_location _returnvalue_rotation _returnvalue_scale) (`KismetMathLibrary.BreakTransform` (`SceneComponent.K2_GetComponentToWorld` (`self.MuzzleScene`))))
  (if (`self.canFire`)
    (bind _returnvalue (`|SpawnActorFromClass` "/Game/MixedHero/Actors/Weapons/arrow_tile.arrow_tile_C" (`KismetMathLibrary.MakeTransform` _returnvalue_location _returnvalue_rotation _returnvalue_scale) "AlwaysSpawn" "OverrideRootScale" null null))
    (`self.K2_AttachToComponent` _returnvalue (`self.MuzzleScene`) "None" "SnapToTarget" "SnapToTarget" "KeepWorld" false)
    (set `self.Arrow` _returnvalue)
    (set `self.ready` true)
    (`self.SetShepreLocation`)))

(fn `SetShepreLocation`
  (`SceneComponent.K2_AttachToComponent` (`self.Sphere`) (`/Game/MixedHero/Controller/BP_HeroMotionController.MotionController` (`self.hand`)) "hand_rSocket" "SnapToTarget" "KeepRelative" "KeepWorld" false))

(fn `UserConstructionScript`)